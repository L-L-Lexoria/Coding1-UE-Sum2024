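; Demo actor for loops and arrays that recolors BP_Key actors one at a time and prints array info on a key press.
; ChangeKeyColor re-calls itself after a Delay, applying colors through dynamic material instances, reshuffling when the index runs out and re-fetching keys when one is invalid.
; The while, recursive, game-loop, Tick and name-listing examples are disconnected, leaving their events empty.
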(event `self.ReceiveBeginPlay`
  ;[0.402 0 0] Event BeginPlay
  (`KismetSystemLibrary.PrintString` "Loops and Lists is Starting" true true (struct :`R` 0.011709 :`G` 0.374677 :`A` 1.0) 5.0)
  (`|ExecutionSequence`
    (:`then_0`
      ;[0.402 0 0] Set-Up for Loops
      (`self.Simple Game Loop`)
      (`self.EnableInput` (`GameplayStatics.GetPlayerController` 0))
      (`self.Recursive Loop`))
    (:`then_1`
      ;[0.402 0 0] Set-Up for Lists
      (bind _outactors (`GameplayStatics.GetAllActorsOfClass` "/Game/Blueprints/BP_Key.BP_Key_C"))
      (set `self.Keys` _outactors)
      (`self.Change Key Color`))))

(event `Simple Game Loop`
  ;[0.402 0.08709 0] Simple Game Loop
)

(event `self.ReceiveTick`
  (params (DeltaSeconds :type "Float (single-precision)"))
  ;[0.402 0.3916 0] Event Tick
)

(event `InputAction|Start While Loop`
  (params (Key :type "Key Structure"))
  ;[0 0.3961 0.02353] The While Loop
)

(event `Recursive Loop`
  ;[0 0.0264 0.3961] Recursive Loop
)

(event `Key|Six`
  (params (Key :type "Key Structure"))
  ;[0.3997 0 0.2265] First Array Test
  (:`Pressed`
    (`self.First Array Test`)))

(event `Key|Five`
  (params (Key :type "Key Structure"))
  ;[0.3997 0 0.2265] First Array Test
  (:`Pressed`
    (`self.List All Names`)))

(event `First Array Test`
  (bind _array (`|MakeArray` "Leia" "Luke" "Han" "Chewie" "Artoo" "Threepio"))
  ;[0.3997 0 0.2265] First Array Test
  (`KismetSystemLibrary.PrintString` (`KismetStringLibrary.Concat_StrStr` "Our array of names has " (`KismetStringLibrary.Conv_IntToString` (`KismetArrayLibrary.Array_Length` _array)) " names in it."))
  (`KismetSystemLibrary.PrintString` (`KismetStringLibrary.Concat_StrStr` "The first name in the array is " (`|GetArrayItem` _array) ".")))

(event `List All Names`
  ;[0.3997 0 0.2265] List All Names
)

(event `Change Key Color`
  (bind _output (`|GetArrayItem` (`self.Keys`) (`self.Color Key Index`)))
  ;[0.3997 0 0.04559] Change Key Color
  ;;[0.3997 0 0.04559] Begin Change Key Color and Branch Test
  (if (or (>= (`self.Color Key Index`) (`KismetArrayLibrary.Array_Length` (`self.Colors`))) (>= (`self.Color Key Index`) (`KismetArrayLibrary.Array_Length` (`self.Keys`))))
    ;;[0.3997 0 0.04559] Shuffle And Reset Colors and Keys
    (`KismetArrayLibrary.Array_Shuffle` (`self.Colors`))
    (`KismetArrayLibrary.Array_Shuffle` (`self.Keys`))
    (set `self.Color Key Index` 0))
  ;;[0.3997 0 0.04559] Test for if Keys is Valid
  (`/Engine/EditorBlueprintResources/StandardMacros.IsValid` _output
    (:`Is Valid`
      ;;[0.3997 0 0.04559] Setting the Color of One Key At A Time
      (bind _returnvalue (`PrimitiveComponent.CreateDynamicMaterialInstance` (`/Game/Blueprints/BP_Key.SM_KeyHead` _output) 0 "/Game/Materials/M_Base.M_Base" "None"))
      (`MaterialInstanceDynamic.SetVectorParameterValue` _returnvalue "Base Color" (`KismetMathLibrary.Conv_ColorToLinearColor` (`|GetArrayItem` (`self.Colors`) (`self.Color Key Index`))))
      ;;[0.3997 0 0.04559] Delay and Restart Loop
      (`/Engine/EditorBlueprintResources/StandardMacros.IncrementInt` (`self.Color Key Index`) :!label _label
        (:`  `
          (`KismetSystemLibrary.Delay` 0.5)
          (`self.Change Key Color`))))
    (:`Is Not Valid`
      ;;[0.3997 0 0.04559] If Invalid, Get All New Actors of Keys and "Re"Set
      (bind _outactors (`GameplayStatics.GetAllActorsOfClass` "/Game/Blueprints/BP_Key.BP_Key_C"))
      ;;[0.3997 0 0.04559] If Array size is 0 (is empty) then do nothing and end loop.
      (if (not (== (`KismetArrayLibrary.Array_Length` _outactors) 0))
        (set `self.Keys` _outactors)
        (goto _label)))))

(fn `UserConstructionScript`)