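; BP_Door is a locked door that the player opens by spending a key.
; When a custom third-person character overlaps its Box, it checks that character's KeyCount.
; With at least one key, it decrements the count, destroys itself and prints the keys left; otherwise it prints a locked message.
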(event `self.Box.OnComponentBeginOverlap`
  (params (OverlappedComponent :type "PrimitiveComponent Object Reference") (OtherActor :type "Actor Object Reference") (OtherComp :type "PrimitiveComponent Object Reference") (OtherBodyIndex :type Integer) (bFromSweep :type Boolean) (SweepResult :type "HitResult Structure (by ref)"))
  (bind _asbp_third_person_character_custom (cast `/Game/Blueprints/BP_ThirdPersonCharacterCustom` OtherActor))
  (bind _keycount (`/Game/Blueprints/BP_ThirdPersonCharacterCustom.keyCount` _asbp_third_person_character_custom))
  (if (> _keycount 0)
    (set `/Game/Blueprints/BP_ThirdPersonCharacterCustom.keyCount` (- _keycount 1) _asbp_third_person_character_custom)
    (`self.K2_DestroyActor`)
    (`KismetSystemLibrary.PrintString` (`KismetStringLibrary.Concat_StrStr` "Door destroyed! You now have " (`KismetStringLibrary.Conv_IntToString` _keycount) " keys left!") true true (struct :`G` 0.66 :`B` 1.0 :`A` 1.0) 5.0)
    (else
      (`KismetSystemLibrary.PrintString` "Door is Locked! Get more Keys!" true true (struct :`R` 0.415444 :`B` 0.000432 :`A` 1.0) 5.0))))

(fn `UserConstructionScript`)