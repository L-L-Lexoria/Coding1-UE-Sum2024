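; BP_FallingPlatform is a platform that falls shortly after the custom third-person character steps on it, then returns to its start.
; An overlap on its collision box starts a one-second warning, then physics simulation drops the platform for five seconds.
; Reset polls until the player no longer overlaps, then disables physics and a timeline lerps the platform back to its saved transform.
; Material swaps and debug prints mark each stage.
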(event `self.ReceiveBeginPlay`
  ;[0.3997 0 0.04559] Begin With Getting World Transform
  (set `self.StartingTransform` (`SceneComponent.K2_GetComponentToWorld` (`self.Platform`))))

(event `self.Collision.OnComponentBeginOverlap`
  (params (OverlappedComponent :type "PrimitiveComponent Object Reference") (OtherActor :type "Actor Object Reference") (OtherComp :type "PrimitiveComponent Object Reference") (OtherBodyIndex :type Integer) (bFromSweep :type Boolean) (SweepResult :type "HitResult Structure (by ref)"))
  ;[0.3997 0 0.2265] Start The Chain For Falling Platform: Did the player overlap the collision box?
  (cast `/Game/Blueprints/BP_ThirdPersonCharacterCustom` OtherActor) ; Did the player step on the platform
  (if (`self.IsReady`)
    (`self.Activate`)))

(event `Activate`
  ;[0 0.0264 0.3961] Activate! Warn the player the platform is about to fall.
  (`KismetSystemLibrary.PrintString` "One Second Left!")
  (set `self.IsReady` false)
  (`PrimitiveComponent.SetMaterial` (`self.Platform`) 0 "/Game/Materials/MI_PlatformReady.MI_PlatformReady")
  (`KismetSystemLibrary.Delay` 1.0)
  (`self.Drop`))

(event `Drop`
  ;[0 0.3961 0.02353] Drop: activate physics to let the platform fall
  (`KismetSystemLibrary.PrintString` "Dropping!")
  (`PrimitiveComponent.SetSimulatePhysics` (`self.Platform`) true)
  (`PrimitiveComponent.SetMaterial` (`self.Platform`) 0 "/Game/Materials/MI_PlatformFalling.MI_PlatformFalling")
  (`KismetSystemLibrary.Delay` 5.0)
  (`self.Reset`))

(event `Reset`
  ;[0.402 0.3916 0] Reset: Check if player is still standing on platform. If not, bring the platform back.
  (bind _returnvalue (`GameplayStatics.GetActorOfClass` "/Game/Blueprints/BP_ThirdPersonCharacterCustom.BP_ThirdPersonCharacterCustom_C"))
  (if (not (`self.IsOverlappingActor` _returnvalue))
    (`KismetSystemLibrary.PrintString` "Resetting!")
    (set `self.ResetTransform` (`SceneComponent.K2_GetComponentToWorld` (`self.Platform`)))
    (`PrimitiveComponent.SetSimulatePhysics` (`self.Platform`) false)
    (`PrimitiveComponent.SetMaterial` (`self.Platform`) 0 "/Game/Materials/MI_PlatformResetting.MI_PlatformResetting")
    (bind (_direction _reset) (`Timeline|ReturnToStart` :!via `PlayFromStart`)
      (:`Update`
        (bind (_returnvalue_location _returnvalue_rotation) (`KismetMathLibrary.BreakTransform` (`KismetMathLibrary.TLerp` (`self.ResetTransform`) (`self.StartingTransform`) _reset)))
        (`SceneComponent.K2_SetWorldLocationAndRotation` (`self.Platform`) _returnvalue_location _returnvalue_rotation false false))
      (:`Finished`
        (set `self.IsReady` true)
        (`PrimitiveComponent.SetMaterial` (`self.Platform`) 0 "/Game/Materials/M_FallingPlatform.M_FallingPlatform")))
    (else
      (`KismetSystemLibrary.Delay` 0.1)
      (`self.Reset`))))

(fn `UserConstructionScript`)